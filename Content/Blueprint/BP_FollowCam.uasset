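; BP_FollowCam is a follow camera actor that tracks the third-person player character's position.
; On BeginPlay it casts the first player character to BP_ThirdPersonCharacter and caches the reference.
; Each Tick, while that reference is valid, it snaps its location to the player's location plus an Offset, with no interpolation, sweep or rotation change.
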(event EventBeginPlay
  ;[0.15 0.15 0.15 0.5] store a reference to the player
  (bind _asbp_third_person_character (Utilities|Casting|CastToBP_ThirdPersonCharacter (Game|GetPlayerCharacter 0)))
  (Variables|Default|SetPlayer%20Reference _asbp_third_person_character))

(event EventTick
  (params (DeltaSeconds :type Float%20%28single-precision%29))
  ;[0.15 0.15 0.15 0.5] set cam position to player's location + an offset
  (Utilities|IsValid (Variables|Default|GetPlayer%20Reference)
    (:Is%20Valid
      (Transformation|SetActorLocation (+ (Transformation|GetActorLocation (Variables|Default|GetPlayer%20Reference)) (Variables|Default|GetOffset)) false false))))

(fn ConstructionScript)