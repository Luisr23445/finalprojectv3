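; BP_goomba is a stompable enemy that moves steadily along a local direction.
; Tick applies a swept local offset from MoveSpeed, MoveDirection and delta time, with no turning logic in the graph.
; Overlapping its top collision launches the third-person character upward, then destroys the goomba after a short delay.
; Overlapping its damage collision calls TakeDamage on that character.
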(event OnComponentBeginOverlap(Damagecollison)
  (params (OverlappedComponent :type Primitive%20Component%20Object%20Reference) (OtherActor :type Actor%20Object%20Reference) (OtherComp :type Primitive%20Component%20Object%20Reference) (OtherBodyIndex :type Integer) (bFromSweep :type Boolean) (SweepResult :type Hit%20Result%20Structure%20%28by%20ref%29))
  ;[0.15 0.15 0.15 0.5] player takes damage when it touches damage collision
  (bind _asbp_third_person_character (Utilities|Casting|CastToBP_ThirdPersonCharacter OtherActor))
  (Default|TakeDamage _asbp_third_person_character))

(event OnComponentBeginOverlap(topcollison)
  (params (OverlappedComponent :type Primitive%20Component%20Object%20Reference) (OtherActor :type Actor%20Object%20Reference) (OtherComp :type Primitive%20Component%20Object%20Reference) (OtherBodyIndex :type Integer) (bFromSweep :type Boolean) (SweepResult :type Hit%20Result%20Structure%20%28by%20ref%29))
  (bind _asbp_third_person_character (Utilities|Casting|CastToBP_ThirdPersonCharacter OtherActor))
  (Character|LaunchCharacter _asbp_third_person_character "0.000000,0.000000,500.000000" false true)
  (Utilities|FlowControl|Delay 0.25)
  (Actor|DestroyActor))

(event EventTick
  (params (DeltaSeconds :type Float%20%28single-precision%29))
  (Transformation|AddActorLocalOffset (* DeltaSeconds (Variables|Default|GetMoveSpeed) (Variables|Default|GetMoveDirection)) true false))

(fn ConstructionScript)