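; BP_thwomp is a falling crusher trap, modeled on a Thwomp, that damages the third-person character.
; When the player enters the CollisionPlayer trigger, a timeline lerps the Thwomp between its BeginPlay location and 420 units below it.
; A DoOnce reset after a delay throttles retriggering, while a separate CollisionDamage overlap calls TakeDamage on the character.
; Older local-offset timeline and InterpToMovement logic remains unconnected.
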(event OnComponentBeginOverlap(CollisionPlayer)
  (params (OverlappedComponent :type Primitive%20Component%20Object%20Reference) (OtherActor :type Actor%20Object%20Reference) (OtherComp :type Primitive%20Component%20Object%20Reference) (OtherBodyIndex :type Integer) (bFromSweep :type Boolean) (SweepResult :type Hit%20Result%20Structure%20%28by%20ref%29))
  (Utilities|Casting|CastToBP_ThirdPersonCharacter OtherActor)
  (Utilities|FlowControl|DoOnce false :!label _label
    (:Completed
      (CallFunction|MoveObject)
      (Utilities|FlowControl|Delay 2.0)
      (goto _label Reset))))

(event OnComponentEndOverlap(CollisionPlayer)
  (params (OverlappedComponent :type Primitive%20Component%20Object%20Reference) (OtherActor :type Actor%20Object%20Reference) (OtherComp :type Primitive%20Component%20Object%20Reference) (OtherBodyIndex :type Integer)))

(event OnComponentBeginOverlap(CollisionDamage)
  (params (OverlappedComponent :type Primitive%20Component%20Object%20Reference) (OtherActor :type Actor%20Object%20Reference) (OtherComp :type Primitive%20Component%20Object%20Reference) (OtherBodyIndex :type Integer) (bFromSweep :type Boolean) (SweepResult :type Hit%20Result%20Structure%20%28by%20ref%29))
  (bind _asbp_third_person_character (Utilities|Casting|CastToBP_ThirdPersonCharacter OtherActor))
  (Default|TakeDamage _asbp_third_person_character))

(event Custom|MoveObject
  (bind _startinglocation (Variables|Default|GetStartingLocation))
  (bind _movetrack (Timeline|T_Move PlayFromStart)
    (:Update
      (Transformation|SetWorldLocation (Variables|Default|GetThwomp) (Math|Vector|Lerp(Vector) _startinglocation (- _startinglocation "0.000000,0.000000,420.000000") _movetrack) false false))))

(event EventBeginPlay
  (Variables|Default|SetStartingLocation (Transformation|GetWorldLocation (Variables|Default|GetThwomp))))

(event EventTick
  (params (DeltaSeconds :type Float%20%28single-precision%29)))

(fn ConstructionScript)