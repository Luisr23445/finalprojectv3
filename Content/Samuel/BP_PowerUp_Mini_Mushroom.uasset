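; Mini mushroom power-up that slides along the X axis and shrinks the player on pickup.
; From BeginPlay, MiniMushroomDirection picks one of two timelines that add or subtract their track value from the X location, with each update looping back to recheck the direction.
; Box overlap by BP_ThirdPersonCharacter calls its Mini function and destroys the mushroom.
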(event OnComponentBeginOverlap(Box)
  (params (OverlappedComponent :type Primitive%20Component%20Object%20Reference) (OtherActor :type Actor%20Object%20Reference) (OtherComp :type Primitive%20Component%20Object%20Reference) (OtherBodyIndex :type Integer) (bFromSweep :type Boolean) (SweepResult :type Hit%20Result%20Structure%20%28by%20ref%29))
  (Development|PrintString "Got mushroom")
  (bind _asbp_third_person_character (Utilities|Casting|CastToBP_ThirdPersonCharacter OtherActor))
  (Default|Mini _asbp_third_person_character)
  (Actor|DestroyActor))

(event Custom|MoveObject
  (if (Variables|Default|GetMiniMushroomDirection) :!label _label
    (if (not (Game|IsActorBeingDestroyed))
      (bind _movetrack (Timeline|Timeline Play)
        (:Update
          (Transformation|SetActorLocationAndRotation (+ (Math|Vector|MakeVector _movetrack 0.0 0.0) (Transformation|GetActorLocation)) "0, 0, 0")
          (goto _label))))
    (elif (not (Game|IsActorBeingDestroyed))
      (bind _movetrack_2 (Timeline|Timeline_0 Play)
        (:Update
          (Transformation|SetActorLocationAndRotation (- (Transformation|GetActorLocation) (Math|Vector|MakeVector _movetrack_2 0.0 0.0)) "0, 0, 0")
          (goto _label))))))

(event EventBeginPlay
  (CallFunction|MoveObject))

(fn ConstructionScript)