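; BP_Fire_Ball is a fireball projectile actor that destroys enemies it touches.
; On BeginPlay, the Move timeline repeatedly offsets the actor along world X from the FireBall component's location, without sweep.
; Box overlap with an "enemy"-tagged actor destroys both actors, then casts that same enemy to BP_ThirdPersonCharacter to decrement NumberOfFireBall, so the count changes only if the enemy is that class.
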(event OnComponentBeginOverlap(Box)
  (params (OverlappedComponent :type Primitive%20Component%20Object%20Reference) (OtherActor :type Actor%20Object%20Reference) (OtherComp :type Primitive%20Component%20Object%20Reference) (OtherBodyIndex :type Integer) (bFromSweep :type Boolean) (SweepResult :type Hit%20Result%20Structure%20%28by%20ref%29))
  (if (Actor|ActorHasTag OtherActor "enemy")
    (Actor|DestroyActor OtherActor)
    (Actor|DestroyActor)
    (bind _asbp_third_person_character (Utilities|Casting|CastToBP_ThirdPersonCharacter OtherActor))
    (Math|Integer|DecrementInt (Variables|/Game/Blueprint/BP_ThirdPersonCharacter.BP_ThirdPersonCharacter_C|GetNumberOfFireBall _asbp_third_person_character))))

(event EventBeginPlay
  (Development|PrintString "Shooting Fire Ball")
  (bind _move (Timeline|Move Play)
    (:Update
      (Transformation|SetActorLocation (+ (Transformation|GetWorldLocation (Variables|Default|GetFireBall)) (Math|Vector|MakeVector _move 0.0 0.0)) false false)
      (Timeline|Move Play))))

(fn ConstructionScript)