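; Mushroom power-up pickup that grows the third-person character on contact.
; A box overlap with BP_ThirdPersonCharacter sets HasPowerUp, calls Grow, prints a debug message and destroys the mushroom.
; The MoveObject event uses a timeline, rate-scaled by TimeToComplete, to move and rotate the actor along SplineRef's spline.
; Nothing in this graph triggers that movement, as the only MoveObject call is disconnected and BeginPlay is empty.
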(event OnComponentBeginOverlap(Box)
  (params (OverlappedComponent :type Primitive%20Component%20Object%20Reference) (OtherActor :type Actor%20Object%20Reference) (OtherComp :type Primitive%20Component%20Object%20Reference) (OtherBodyIndex :type Integer) (bFromSweep :type Boolean) (SweepResult :type Hit%20Result%20Structure%20%28by%20ref%29))
  (bind _asbp_third_person_character (Utilities|Casting|CastToBP_ThirdPersonCharacter OtherActor))
  (Variables|/Game/Blueprint/BP_ThirdPersonCharacter.BP_ThirdPersonCharacter_C|SetHasPowerUp _asbp_third_person_character true)
  (Default|Grow _asbp_third_person_character)
  (Development|PrintString "Got the mushroom")
  (Actor|DestroyActor))

(event Custom|MoveObject
  (bind _splineref (Variables|Default|GetSplineRef))
  (bind _spline (Variables|/Game/Samuel/BP_Spline_Mushroom.BP_Spline_Mushroom_C|GetSpline _splineref))
  (Components|Timeline|SetPlayRate (Variables|Default|GetT_Move) (/ 1.0 (Variables|Default|GetTimeToComplete)))
  (bind _movetrack (Timeline|T_Move Play)
    (:Update
      (Transformation|SetActorLocationAndRotation (Spline|GetLocationatDistanceAlongSpline _spline (Math|Float|Lerp 0.0 (Spline|GetSplineLength _spline) _movetrack) "World") (Spline|GetRotationatDistanceAlongSpline _spline (Math|Float|Lerp 0.0 (Spline|GetSplineLength _spline) _movetrack) "World")))))

(event EventBeginPlay)

(fn ConstructionScript)