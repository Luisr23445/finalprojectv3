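; BP_thwomp_trigger is a trigger volume meant to set off a Thwomp when the third-person character overlaps its collision box.
; On overlap it prints a debug message, then plays a Timeline that writes Alpha directly as the yaw of the Thwomp component.
; The Thwomp reference comes from casting the same overlapping actor already cast as the character, so the Timeline is normally never reached.
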(event OnComponentBeginOverlap(PlayerCollissionBox)
  (params (OverlappedComponent :type Primitive%20Component%20Object%20Reference) (OtherActor :type Actor%20Object%20Reference) (OtherComp :type Primitive%20Component%20Object%20Reference) (OtherBodyIndex :type Integer) (bFromSweep :type Boolean) (SweepResult :type Hit%20Result%20Structure%20%28by%20ref%29))
  (Utilities|Casting|CastToBP_ThirdPersonCharacter OtherActor)
  (Development|PrintString "Trigger_Thwomp")
  (bind _asbp_thwomp (Utilities|Casting|CastToBP_thwomp OtherActor))
  (bind _alpha (Timeline|Timeline Play)
    (:Update
      (bind _output_get (Variables|Default|SetAlpha _alpha))
      (Transformation|SetRelativeRotation (Variables|/Game/Samuel/BP_thwomp.BP_thwomp_C|GetThwomp _asbp_thwomp) (Math|Rotator|MakeRotator 0.0 0.0 _output_get) false false))))

(event EventBeginPlay)

(event Collision|EventActorBeginOverlap
  (params (OtherActor :type Actor%20Object%20Reference)))

(event EventTick
  (params (DeltaSeconds :type Float%20%28single-precision%29)))

(fn ConstructionScript)